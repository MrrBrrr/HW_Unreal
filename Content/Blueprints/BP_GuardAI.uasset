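; BP_GuardAI is a guard pawn that wanders endlessly between random navigable points.
; SpawnNextRandomTarget replaces AimActor with a scaled-down, re-skinned BP_Projectile at a random reachable point near the guard, serving as the move target.
; AI MoveTo heads for that marker and picks a new one on success or failure.
; DrawTrace, uncalled here, line-traces toward a location and respawns the target via ChangeDestination when the projectile cast fails, without reissuing the move.
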(event `self.ReceiveBeginPlay`
  (`self.Spawn Next Random Target`)
  (`self.MoveToAimTarget`))

(event `MoveToAimTarget`
  (`|AIMoveTo` self (0.0 0.0 0.0) (`self.AimActor`)
    (:`OnSuccess`
      _)
    (:`OnFail`
      _))
  (`self.Spawn Next Random Target`)
  (`self.MoveToAimTarget`))

(fn `ChangeDestination`
  (params (OtherActor :type "Actor Object Reference"))
  (if (not (== OtherActor (`self.AimActor`)))
    (`self.Spawn Next Random Target`)))

(fn `Destroy if Valid`
  (params (Object :type "Actor Object Reference"))
  (if (`KismetSystemLibrary.IsValid` Object)
    (`self.K2_DestroyActor` Object)
    (return)
    (else
      (return))))

(fn `Draw Trace`
  (params (`Target Location` :type "Vector Structure"))
  (locals (`Object Types` :type "Array of EObjectTypeQuery Enum"))
  (bind _outhit (`KismetSystemLibrary.LineTraceSingleForObjects` :`Start` (- (`SceneComponent.K2_GetComponentLocation` (`self.CapsuleComponent`)) (0.0 0.0 -50.0)) :`End` `Target Location` :`ObjectTypes` (`local.Object Types`) :`DrawDebugType` "ForOneFrame"))
  (bind _asbp_projectile (cast `/Game/Blueprints/Lecture15_Scout/BP_Projectile` (`.HitActor` (`GameplayStatics.BreakHitResult` _outhit)))
    (:`CastFailed`
      (`self.ChangeDestination` _asbp_projectile))))

(fn `Spawn Next Random Target`
  (returns (AimSpawnLocation :type "Vector Structure"))
  (locals (AimActorSpawnLocation :type "Vector Structure"))
  (`self.Destroy if Valid` (`self.AimActor`))
  (bind _output_get (set `local.AimActorSpawnLocation` (`NavigationSystemV1.K2_GetRandomLocationInNavigableRadius` (`self.K2_GetActorLocation`) 1000.0 null null)))
  (bind _returnvalue (`|SpawnActorFromClass` "/Game/Blueprints/Lecture15_Scout/BP_Projectile.BP_Projectile_C" (`KismetMathLibrary.MakeTransform` _output_get (struct) (0.3 0.3 0.3)) "Undefined" "OverrideRootScale" null null))
  (`PrimitiveComponent.SetMaterial` (`/Game/Blueprints/Lecture15_Scout/BP_Projectile.StaticMesh` _returnvalue) 0 "/Engine/MapTemplates/Materials/BasicAsset03.BasicAsset03")
  (set `self.AimActor` _returnvalue)
  (return (`local.AimActorSpawnLocation`)))

(fn `UserConstructionScript`)