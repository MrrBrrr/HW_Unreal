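; Arkanoid projectile actor that travels along its forward vector and bounces off whatever it hits.
; Each tick it moves with a swept offset, scaling its Speed by the ProjectileSpeedFactor from the Arkanoid game state cached at BeginPlay.
; On hit it reflects its forward vector about the surface normal, normalizes it in 2D and rotates to face that direction, keeping bounces planar.
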(event `self.ReceiveBeginPlay`
  (bind _asbp_arkanoid_game_state (cast `/Game/Blueprints/Arkanoid/BP_ArkanoidGameState` (`GameplayStatics.GetGameState`)))
  (set `self.As BP Arkanoid Game State` _asbp_arkanoid_game_state))

(event `self.ReceiveTick`
  (params (DeltaSeconds :type "Float (single-precision)"))
  (`self.K2_AddActorWorldOffset` (* (`self.GetActorForwardVector`) (* DeltaSeconds (`self.Speed`) (`/Game/Blueprints/Arkanoid/BP_ArkanoidGameState.ProjectileSpeedFactor` (`self.As BP Arkanoid Game State`)))) true))

(event `self.ReceiveHit`
  (params (MyComp :type "PrimitiveComponent Object Reference") (Other :type "Actor Object Reference") (OtherComp :type "PrimitiveComponent Object Reference") (bSelfMoved :type Boolean) (HitLocation :type "Vector Structure") (HitNormal :type "Vector Structure") (NormalImpulse :type "Vector Structure") (Hit :type "HitResult Structure (by ref)"))
  (`self.K2_SetActorRotation` (`KismetMathLibrary.MakeRotFromX` (`KismetMathLibrary.Vector_Normal2D` (`KismetMathLibrary.GetReflectionVector` (`self.GetActorForwardVector`) HitNormal) 0.1))))

(fn `UserConstructionScript`)