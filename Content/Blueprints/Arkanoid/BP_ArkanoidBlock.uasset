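; Arkanoid brick actor that takes two hits from BP_ArkanoidProjectile to destroy.
; The first hit swaps the mesh material.
; The second usually spawns a BP_Bonus (80% chance, though the inline comment says 50%), with type and emission color supplied by the game state.
; It then has the game state run the end-game check and add score before destroying itself.
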(event `self.ReceiveBeginPlay`
  (bind _asbp_arkanoid_game_state (cast `/Game/Blueprints/Arkanoid/BP_ArkanoidGameState` (`GameplayStatics.GetGameState`)))
  (set `self.As BP Arkanoid Game State` _asbp_arkanoid_game_state))

(event `self.ReceiveHit`
  (params (MyComp :type "PrimitiveComponent Object Reference") (Other :type "Actor Object Reference") (OtherComp :type "PrimitiveComponent Object Reference") (bSelfMoved :type Boolean) (HitLocation :type "Vector Structure") (HitNormal :type "Vector Structure") (NormalImpulse :type "Vector Structure") (Hit :type "HitResult Structure (by ref)"))
  (cast `/Game/Blueprints/Arkanoid/BP_ArkanoidProjectile` Other)
  (if (`self.IsFirstHit`)
    (set `self.IsFirstHit` false)
    (`PrimitiveComponent.SetMaterial` (`self.StaticMesh`) 0 "/Engine/EngineDebugMaterials/LightingModels/M_TextureDefinedSpecularReflecti.M_TextureDefinedSpecularReflecti")
    (else
      (`|ExecutionSequence`
        (:`then_0`
          ;[1 1 1] 50% to spawn bonus
          (if (> (`KismetMathLibrary.RandomFloatInRange` 0.0 1.0) 0.2)
            (bind (_nextcolor _nexttype) (`/Game/Blueprints/Arkanoid/BP_ArkanoidGameState.NextBonusParams` (`self.As BP Arkanoid Game State`)))
            (bind _returnvalue (`|SpawnActorFromClass` "/Game/Blueprints/Arkanoid/BP_Bonus.BP_Bonus_C" (`SceneComponent.K2_GetComponentToWorld` (`self.Box`)) "Undefined" "OverrideRootScale" null _nexttype null))
            (`/Game/Blueprints/Arkanoid/BP_Bonus.SetEmissionColor` _returnvalue _nextcolor)))
        (:`then_1`
          (`/Game/Blueprints/Arkanoid/BP_ArkanoidGameState.EndGameCheck` (`self.As BP Arkanoid Game State`)))
        (:`then_2`
          (`/Game/Blueprints/Arkanoid/BP_ArkanoidGameState.Add Score` (`self.As BP Arkanoid Game State`) 1))
        (:`then_3`
          (`self.K2_DestroyActor`))))))

(fn `UserConstructionScript`)