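; BP_Bonus is an Arkanoid pickup that grants an effect when it overlaps the player's platform.
; It moves along its forward vector each tick with a swept offset at its Speed.
; On platform overlap, BonusType selects between spawning a projectile through the platform or increasing the speed timer in BP_ArkanoidGameState, then the actor destroys itself.
; SetEmissionColor recolors its Emission light.
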(event `self.ReceiveBeginPlay`
  (`SceneComponent.K2_SetWorldRotation` (`self.StaticMesh`) (struct :`Yaw` 180.0) false false))

(event `self.ReceiveActorBeginOverlap`
  (params (OtherActor :type "Actor Object Reference"))
  (bind _asbp_arkanoid_platform (cast `/Game/Blueprints/Arkanoid/BP_ArkanoidPlatform` OtherActor))
  (switch `/Game/Blueprints/Arkanoid/EBonusTypes` (`self.BonusType`)
    (:`NewEnumerator0`
      (`/Game/Blueprints/Arkanoid/BP_ArkanoidPlatform.Spawn Projectile Event` _asbp_arkanoid_platform))
    (:`NewEnumerator1`
      (bind _asbp_arkanoid_game_state (cast `/Game/Blueprints/Arkanoid/BP_ArkanoidGameState` (`GameplayStatics.GetGameState`)))
      (`/Game/Blueprints/Arkanoid/BP_ArkanoidGameState.Increase Speed Timer` _asbp_arkanoid_game_state)))
  (`self.K2_DestroyActor`))

(event `self.ReceiveTick`
  (params (DeltaSeconds :type "Float (single-precision)"))
  (`self.K2_AddActorWorldOffset` (* (`self.GetActorForwardVector`) (* DeltaSeconds (`self.Speed`))) true))

(fn `SetEmissionColor`
  (params (EmissionColor :type "LinearColor Structure"))
  (`LightComponent.SetLightColor` (`self.Emission`) EmissionColor false))

(fn `UserConstructionScript`)