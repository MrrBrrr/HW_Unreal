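; BP_ArkanoidBlocks builds the grid of blocks for an Arkanoid-style game.
; Its construction script adds an X-by-Y grid of child actor components spaced by Padding along negative X and positive Y, incrementing BlocksCount for each.
; On BeginPlay it passes BlocksCount to BP_ArkanoidGameState.
; The overlap, tick and hit events are empty.
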(event `self.ReceiveBeginPlay`
  (bind _asbp_arkanoid_game_state (cast `/Game/Blueprints/Arkanoid/BP_ArkanoidGameState` (`GameplayStatics.GetGameState`)))
  (`/Game/Blueprints/Arkanoid/BP_ArkanoidGameState.SetBlocksCount` _asbp_arkanoid_game_state (`self.BlocksCount`)))

(event `self.ReceiveActorBeginOverlap`
  (params (OtherActor :type "Actor Object Reference")))

(event `self.ReceiveHit`
  (params (MyComp :type "PrimitiveComponent Object Reference") (Other :type "Actor Object Reference") (OtherComp :type "PrimitiveComponent Object Reference") (bSelfMoved :type Boolean) (HitLocation :type "Vector Structure") (HitNormal :type "Vector Structure") (NormalImpulse :type "Vector Structure") (Hit :type "HitResult Structure (by ref)")))

(fn `UserConstructionScript`
  (for _index (range (+ (`self.X`) 1))
    (for _index_2 (range (+ (`self.Y`) 1))
      (`AddComponent|NODE_AddChildActorComponent-0` :`RelativeTransform` (`KismetMathLibrary.MakeTransform` (`KismetMathLibrary.MakeVector` (`KismetMathLibrary.Conv_IntToDouble` (* (* _index (`self.Padding`)) -1)) (`KismetMathLibrary.Conv_IntToDouble` (* _index_2 (`self.Padding`))))))
      (`/Engine/EditorBlueprintResources/StandardMacros.IncrementInt` (`self.BlocksCount`)))))