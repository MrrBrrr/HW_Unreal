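; BP_EndGameTrigger is the Arkanoid trigger actor that removes projectiles and bonuses that overlap it.
; On overlap it destroys a BP_ArkanoidProjectile and notifies its Platform reference through OnProjectileDestroy.
; A separate sequence branch destroys any overlapping BP_Bonus.
; BeginPlay caches the BP_ArkanoidGameState, though the graphs shown do not use it afterwards.
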(event `self.ReceiveBeginPlay`
  (bind _asbp_arkanoid_game_state (cast `/Game/Blueprints/Arkanoid/BP_ArkanoidGameState` (`GameplayStatics.GetGameState`)))
  (set `self.As BP Arkanoid Game State` _asbp_arkanoid_game_state))

(event `self.ReceiveActorBeginOverlap`
  (params (OtherActor :type "Actor Object Reference"))
  (`|ExecutionSequence`
    (:`then_0`
      (bind _asbp_arkanoid_projectile (cast `/Game/Blueprints/Arkanoid/BP_ArkanoidProjectile` OtherActor))
      (`self.K2_DestroyActor` _asbp_arkanoid_projectile)
      (`/Game/Blueprints/Arkanoid/BP_ArkanoidPlatform.On Projectile Destroy` (`self.Platform`)))
    (:`then_1`
      (bind _asbp_bonus (cast `/Game/Blueprints/Arkanoid/BP_Bonus` OtherActor))
      (`self.K2_DestroyActor` _asbp_bonus))))

(fn `UserConstructionScript`)