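; Arkanoid game state that tracks score, remaining blocks and the timed projectile speed bonus.
; The speed bonus raises the projectile speed factor, then a looping one-second timer counts down and restores it.
; A weighted random roll picks the next bonus color and type.
; The end check decrements the block count and pauses the game at zero, with visibility values flagging bonus and game-over states.
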(event `Increase Speed Timer`
  (set `self.BounsTime` (`self.DefaultBounsTime`))
  (bind _returnvalue (`KismetSystemLibrary.K2_SetTimerDelegate` (delegate `MainTimerEvent`) 1.0 true))
  (set `self.Timer` _returnvalue)
  (set `self.ProjectileSpeedFactor` 1.5)
  (set `self.IsSpeedBonusActive` "Visible"))

(event `MainTimerEvent`
  (bind _result (`/Engine/EditorBlueprintResources/StandardMacros.DecrementInt` (`self.BounsTime`))
    (:`  `
      (if (< _result 1)
        (`KismetSystemLibrary.K2_ClearAndInvalidateTimerHandle` (`self.Timer`))
        (set `self.ProjectileSpeedFactor` 1.0)
        (set `self.BounsTime` (`self.DefaultBounsTime`))
        (set `self.IsSpeedBonusActive` "Hidden")))))

(event `Add Score`
  (params (Bonus :type Integer))
  (set `self.Score` (+ Bonus (`self.Score`))))

(fn `EndGameCheck`
  (bind _result (`/Engine/EditorBlueprintResources/StandardMacros.DecrementInt` (`self.BlocksCount`))
    (:`  `
      (if (< _result 1)
        (set `self.IsGameEnded` "Visible")
        (`GameplayStatics.SetGamePaused` true)))))

(fn `GetBounsTimer`
  (returns (TimePlayed :type Integer))
  (return (`self.BounsTime`)))

(fn `NextBonusParams`
  (returns (NextColor :type "LinearColor Structure") (NextType :type "/Game/Blueprints/Arkanoid/EBonusTypes Enum"))
  (locals (PurpleColor :type "LinearColor Structure" :default (struct :`R` 0.59975 :`B` 1.0 :`A` 1.0)) (GreenColor :type "LinearColor Structure" :default (struct :`R` 0.461438 :`G` 1.0 :`A` 1.0)))
  (if (< (`KismetMathLibrary.RandomFloatInRange` 0.0 1.0) 0.8)
    (return (`local.PurpleColor`) "NewEnumerator0")
    (else
      (return (`local.GreenColor`) "NewEnumerator1"))))

(fn `SetBlocksCount`
  (params (BlocksCount :type Integer))
  (set `self.BlocksCount` BlocksCount))

(fn `UserConstructionScript`)