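; Player paddle for an Arkanoid game that slides sideways on the MoveRight axis and launches projectiles.
; Movement is swept and frame-rate independent, scaled by Speed and the game state's ProjectileSpeedFactor.
; A projectile spawns just in front of the mesh at begin play, incrementing the game state's ProjectileCount.
; OnProjectileDestroy decrements that count and spawns a replacement when none remain.
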(event `self.ReceiveBeginPlay`
  (bind _asbp_arkanoid_game_state (cast `/Game/Blueprints/Arkanoid/BP_ArkanoidGameState` (`GameplayStatics.GetGameState`)))
  (set `self.As BP Arkanoid Game State` _asbp_arkanoid_game_state)
  (`self.Spawn Projectile Event`))

(event `InputAxis|MoveRight`
  (params (AxisValue :type "Float (single-precision)"))
  (`self.K2_AddActorLocalOffset` (`KismetMathLibrary.MakeVector` 0.0 (* AxisValue (`self.Speed`) (`/Game/Blueprints/Arkanoid/BP_ArkanoidGameState.ProjectileSpeedFactor` (`self.As BP Arkanoid Game State`)) (`GameplayStatics.GetWorldDeltaSeconds`))) true))

(event `Spawn Projectile Event`
  (bind (_returnvalue_x _returnvalue_y _returnvalue_z) (`KismetMathLibrary.BreakVector` (`SceneComponent.K2_GetComponentLocation` (`self.StaticMesh`))))
  (bind _returnvalue (`|SpawnActorFromClass` "/Game/Blueprints/Arkanoid/BP_ArkanoidProjectile.BP_ArkanoidProjectile_C" (`KismetMathLibrary.MakeTransform` (`KismetMathLibrary.MakeVector` (+ _returnvalue_x 30.0) _returnvalue_y _returnvalue_z) (struct :`Yaw` 12.0) (0.5 0.5 0.5)) "AdjustIfPossibleButDontSpawnIfColliding" "OverrideRootScale" null null))
  (`/Engine/EditorBlueprintResources/StandardMacros.IsValid` _returnvalue
    (:`Is Valid`
      (`/Engine/EditorBlueprintResources/StandardMacros.IncrementInt` (`/Game/Blueprints/Arkanoid/BP_ArkanoidGameState.ProjectileCount` (`self.As BP Arkanoid Game State`))))))

(event `On Projectile Destroy`
  (bind _result (`/Engine/EditorBlueprintResources/StandardMacros.DecrementInt` (`/Game/Blueprints/Arkanoid/BP_ArkanoidGameState.ProjectileCount` (`self.As BP Arkanoid Game State`)))
    (:`  `
      (if (< _result 1)
        (`self.Spawn Projectile Event`)))))

(fn `UserConstructionScript`)