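; Game mode for a rock game that starts the match, spawns rocks at random map positions and forwards end/restart events to BP_GameState.
; Process(CurrentTime) periodically adds a rock and raises difficulty, which scales each new rock's speed.
; A second period triggers an announced "Crazy Cubes" wave of faster rocks, removed after a delay.
; IsCppRock switches between BP_Rock and BP_Rock_Danger, though wave cleanup only destroys the latter.
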(event `self.ReceiveBeginPlay`
  (bind _asbp_game_state (cast `/Game/Blueprints/Rocks/BP_GameState` (`GameplayStatics.GetGameState`)))
  (bind _output_get (set `self.As BP Game State` _asbp_game_state))
  (`/Game/Blueprints/Rocks/BP_GameState.StartGame` _output_get)
  (for _ (range 10)
    (`self.Spawn Rock` 1.0)))

(event `Process`
  (params (CurrentTime :type Integer))
  (`|ExecutionSequence`
    (:`then_0`
      (if (== (mod CurrentTime (`self.SecondsPeriod`)) 0)
        (`self.Spawn Rock` 1.0)
        (`/Game/Blueprints/Rocks/BP_GameState.IncreaseDifficulty` (`self.As BP Game State`))))
    (:`then_1`
      (if (== (mod CurrentTime (`self.FastRockSecondsPeriod`)) 0)
        (`KismetSystemLibrary.PrintString` (`KismetStringLibrary.Concat_StrStr` " \n" " \n" " \n" "  \n" (`self.CrazyCubesComeText`)) true true (struct :`R` 0.104583 :`G` 1.0 :`A` 1.0) 10.0)
        (set `/Game/Blueprints/Rocks/BP_GameState.IsCrazyCubesSpawned` true (`self.As BP Game State`))
        (for _ (range 6)
          (`self.Spawn Rock` 1.1))
        (`KismetSystemLibrary.Delay` (`KismetMathLibrary.Conv_IntToDouble` (`self.DestroyAllFastRock`)))
        (for _array_element (`self.FastRocks`)
          (`self.K2_DestroyActor` _array_element))
        (if (`self.IsCppRock`)
          (`KismetArrayLibrary.Array_Clear` (`self.CppFastRocks`))
          (else
            (`KismetArrayLibrary.Array_Clear` (`self.FastRocks`))))
        (`KismetSystemLibrary.PrintString` (`KismetStringLibrary.Concat_StrStr` " \n" " \n" " \n" "  \n" (`self.CrazyCubesGoneText`)) true true (struct :`R` 0.348958 :`G` 0.586263 :`B` 1.0 :`A` 1.0) 3.0)
        (set `/Game/Blueprints/Rocks/BP_GameState.IsCrazyCubesSpawned` true (`self.As BP Game State`))))))

(event `EndEvent`
  (`/Game/Blueprints/Rocks/BP_GameState.EndGameEvent` (`self.As BP Game State`)))

(event `RestartEvent`
  (`/Game/Blueprints/Rocks/BP_GameState.RestartGameEvent` (`self.As BP Game State`)))

(fn `Spawn Rock`
  (params (SpeedRatio :type "Float (double-precision)"))
  (locals (MapEdgeCoordinate :type "Float (double-precision)" :default 1900.0) (RockHigh :type "Float (double-precision)" :default 100.0))
  (bind _mapedgecoordinate (`local.MapEdgeCoordinate`))
  (bind _mapedgecoordinate_2 (`local.MapEdgeCoordinate`))
  (bind _returnvalue (* -1 _mapedgecoordinate_2))
  (bind _returnvalue_2 (* -1 _mapedgecoordinate))
  (if (`self.IsCppRock`)
    (bind _returnvalue_3 (`|SpawnActorFromClass` "/Game/Blueprints/Rocks/BP_Rock.BP_Rock_C" (`KismetMathLibrary.MakeTransform` (`KismetMathLibrary.MakeVector` (`KismetMathLibrary.RandomFloatInRange` _returnvalue_2 _mapedgecoordinate) (`KismetMathLibrary.RandomFloatInRange` _returnvalue_2 _mapedgecoordinate) (`local.RockHigh`))) "Undefined" "OverrideRootScale" null null))
    (set `BbRock.Speed` (* (`KismetMathLibrary.Conv_IntToDouble` (`/Game/Blueprints/Rocks/BP_GameState.GetDifficulty` (`self.As BP Game State`))) SpeedRatio) _returnvalue_3)
    (if (> SpeedRatio 1.0)
      (`KismetArrayLibrary.Array_Add` (`self.CppFastRocks`)))
    (else
      (bind _returnvalue_4 (`|SpawnActorFromClass` "/Game/Blueprints/Rocks/BP_Rock_Danger.BP_Rock_Danger_C" (`KismetMathLibrary.MakeTransform` (`KismetMathLibrary.MakeVector` (`KismetMathLibrary.RandomFloatInRange` _returnvalue _mapedgecoordinate_2) (`KismetMathLibrary.RandomFloatInRange` _returnvalue _mapedgecoordinate_2) (`local.RockHigh`))) "AdjustIfPossibleButAlwaysSpawn" "OverrideRootScale" null null))
      (set `/Game/Blueprints/Rocks/BP_Rock_Danger.Speed` (* (* (`KismetMathLibrary.Conv_IntToDouble` (`/Game/Blueprints/Rocks/BP_GameState.GetDifficulty` (`self.As BP Game State`))) SpeedRatio) (`/Game/Blueprints/Rocks/BP_Rock_Danger.Speed` _returnvalue_4)) _returnvalue_4)
      (if (> SpeedRatio 1.0)
        (`KismetArrayLibrary.Array_Add` (`self.FastRocks`))))))

(fn `UserConstructionScript`)