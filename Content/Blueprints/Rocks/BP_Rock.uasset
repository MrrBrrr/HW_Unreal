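; BP_Rock is a rock hazard that kills the female player character and ends the game event.
; On BeginPlay, TurnToTarget snaps its forward axis toward the first player's pawn using a flattened 2D direction, with no later re-aiming.
; A custom event takes another actor, destroys it if it is a BP_FemaleCharacter, then calls EndEvent on BP_GameMode.
; Nothing in these graphs moves the rock or triggers that event.
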(event `self.ReceiveBeginPlay`
  (`self.TurnToTarget` (`GameplayStatics.GetPlayerPawn` 0)))

(event `self.ReceiveTick`
  (params (DeltaSeconds :type "Float (single-precision)")))

(event `CustomEvent`
  (params (OtherActor :type "Actor Object Reference"))
  (bind _asbp_female_character (cast `/Game/ThirdPersonBP/Blueprints/BP_FemaleCharacter` OtherActor))
  (`self.K2_DestroyActor` _asbp_female_character)
  (bind _asbp_game_mode (cast `/Game/Blueprints/Rocks/BP_GameMode` (`GameplayStatics.GetGameMode`)))
  (`/Game/Blueprints/Rocks/BP_GameMode.EndEvent` _asbp_game_mode))

(fn `UserConstructionScript`)