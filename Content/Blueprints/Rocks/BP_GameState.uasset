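; Game state for the Rocks game that tracks time played, difficulty and the end and restart of a run.
; A looping one-second timer awards each player score scaled by difficulty, boosted while crazy cubes are spawned, and passes elapsed time to BP_GameMode for processing.
; Game end stops the timer, submits scores to BP_GameInstance as high-score candidates and decrements lives per player.
; Restart reloads the current level if lives remain.
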(event `StartGame`
  (bind _returnvalue (`KismetSystemLibrary.K2_SetTimerDelegate` (delegate `MainTimerEvent`) 1.0 true))
  (set `self.Timer` _returnvalue)
  (set `self.IsGameEnded` false))

(event `MainTimerEvent`
  (`/Engine/EditorBlueprintResources/StandardMacros.IncrementInt` (`self.TimePlayed`)
    (:`  `
      (for _array_element (`self.PlayerArray`)
        (bind _asbp_player_state (cast `/Game/ThirdPersonBP/Blueprints/BP_PlayerState` _array_element))
        (if (`self.IsCrazyCubesSpawned`)
          (`/Game/ThirdPersonBP/Blueprints/BP_PlayerState.AddPlayerScore` _asbp_player_state (* (`self.Difficulty`) 5))
          (else
            (`/Game/ThirdPersonBP/Blueprints/BP_PlayerState.AddPlayerScore` _asbp_player_state (`self.Difficulty`)))))
      (bind _asbp_game_mode (cast `/Game/Blueprints/Rocks/BP_GameMode` (`GameplayStatics.GetGameMode`)))
      (`/Game/Blueprints/Rocks/BP_GameMode.Process` _asbp_game_mode (`self.TimePlayed`)))))

(event `EndGameEvent`
  (`KismetSystemLibrary.K2_ClearAndInvalidateTimerHandle` (`self.Timer`))
  (set `self.IsGameEnded` true)
  (bind _asbp_game_instance (cast `/Game/Blueprints/Rocks/BP_GameInstance` (`GameplayStatics.GetGameInstance`)))
  (for _array_element (`self.PlayerArray`)
    (bind _asbp_player_state (cast `/Game/ThirdPersonBP/Blueprints/BP_PlayerState` _array_element))
    (`/Game/Blueprints/Rocks/BP_GameInstance.SetHighestScore` _asbp_game_instance (`/Game/ThirdPersonBP/Blueprints/BP_PlayerState.GetPlayerScore` _asbp_player_state))
    (bind _result (`/Engine/EditorBlueprintResources/StandardMacros.DecrementInt` (`/Game/Blueprints/Rocks/BP_GameInstance.Lives` _asbp_game_instance))
      (:`  `
        (set `self.Lives` _result)))))

(event `RestartGameEvent`
  (bind _asbp_game_instance (cast `/Game/Blueprints/Rocks/BP_GameInstance` (`GameplayStatics.GetGameInstance`)))
  (if (`/Game/Blueprints/Rocks/BP_GameInstance.IsLiveRemaining` _asbp_game_instance)
    (bind _returnvalue (`GameplayStatics.GetCurrentLevelName` true))
    (`GameplayStatics.OpenLevel` (`KismetStringLibrary.Conv_StringToName` _returnvalue))))

(fn `GetDifficulty`
  (returns (Difficulty :type Integer))
  (return (`self.Difficulty`)))

(fn `GetIsGameEnded`
  (returns (IsGameEnded :type Boolean))
  (return (`self.IsGameEnded`)))

(fn `GetTimePlayed`
  (returns (TimePlayed :type Integer))
  (return (`self.TimePlayed`)))

(fn `IncreaseDifficulty`
  (`/Engine/EditorBlueprintResources/StandardMacros.IncrementInt` (`self.Difficulty`)))

(fn `UserConstructionScript`)