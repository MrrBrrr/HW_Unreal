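; BP_Rock_Danger is a moving hazard rock that destroys the player character and ends the game on contact.
; On BeginPlay it turns toward the player pawn's position, then Tick sweeps it forward at Speed without homing.
; A hit on BP_FemaleCharacter destroys it and calls EndEvent on BP_GameMode.
; Any other hit bounces the rock by reflecting its heading off the surface normal, flattened to 2D.
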(event `self.ReceiveBeginPlay`
  (`self.TurnToTarget` (`GameplayStatics.GetPlayerPawn` 0)))

(event `self.ReceiveTick`
  (params (DeltaSeconds :type "Float (single-precision)"))
  (`self.K2_AddActorWorldOffset` (* (`self.GetActorForwardVector`) (* DeltaSeconds (`self.Speed`))) true))

(event `self.ReceiveHit`
  (params (MyComp :type "PrimitiveComponent Object Reference") (Other :type "Actor Object Reference") (OtherComp :type "PrimitiveComponent Object Reference") (bSelfMoved :type Boolean) (HitLocation :type "Vector Structure") (HitNormal :type "Vector Structure") (NormalImpulse :type "Vector Structure") (Hit :type "HitResult Structure (by ref)"))
  (bind _asbp_female_character (cast `/Game/ThirdPersonBP/Blueprints/BP_FemaleCharacter` Other)
    (:`then`
      (`self.K2_DestroyActor` _asbp_female_character)
      (bind _asbp_game_mode (cast `/Game/Blueprints/Rocks/BP_GameMode` (`GameplayStatics.GetGameMode`)))
      (`/Game/Blueprints/Rocks/BP_GameMode.EndEvent` _asbp_game_mode))
    (:`CastFailed`
      (`self.K2_SetActorRotation` (`KismetMathLibrary.MakeRotFromX` (`KismetMathLibrary.Vector_Normal2D` (`KismetMathLibrary.GetReflectionVector` (`self.GetActorForwardVector`) HitNormal)))))))

(fn `UserConstructionScript`)