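; BP_Controller is an overlap-driven actor that cycles the material of a referenced actor while something overlaps it.
; BeginPlay creates a looping half-second timer and immediately pauses it; overlap begin and end unpause and pause it, also opening and closing a Gate.
; Each timer tick passes through the Gate and sends the next Collection entry to the target's ChangeMaterial, wrapping the incrementing index with modulo.
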(event `self.ReceiveBeginPlay`
  (bind _returnvalue (`KismetSystemLibrary.K2_SetTimerDelegate` (delegate `ChangeMaterial`) 0.5 true))
  (`KismetSystemLibrary.K2_PauseTimerHandle` _returnvalue))

(event `ChangeMaterial`
  (bind _collection_ (`self.Collection `))
  (`/Engine/EditorBlueprintResources/StandardMacros.Gate` true :!label _label
    (:`Exit`
      (`/Game/Blueprints/Lecture10/BP_Target.ChangeMaterial` (`self.ActorToChangeMaterial`) (`|GetArrayItem` _collection_ (mod (`self.CollectionIndex`) (`KismetArrayLibrary.Array_Length` _collection_))))
      (`/Engine/EditorBlueprintResources/StandardMacros.IncrementInt` (`self.CollectionIndex`)))))

(event `self.ReceiveActorBeginOverlap`
  (params (OtherActor :type "Actor Object Reference"))
  (`KismetSystemLibrary.K2_UnPauseTimerHandle` (stale `self.ReceiveBeginPlay` _returnvalue))
  (goto _label :!via `Open`))

(event `self.ReceiveActorEndOverlap`
  (params (OtherActor :type "Actor Object Reference"))
  (`KismetSystemLibrary.K2_PauseTimerHandle` (stale `self.ReceiveBeginPlay` _returnvalue))
  (goto _label :!via `Close`))

(fn `UserConstructionScript`)