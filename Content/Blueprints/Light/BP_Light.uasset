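; BP_Light is a light actor that cycles through a set of colors and displays the current color's name as text.
; A looping timer started on BeginPlay increments a counter, offsets it by ColorIndex and wraps it to the color map's length.
; The result becomes an ELightColor key into color and name maps, whose values SetColor applies to the PointLight and TextRender.
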(event `self.ReceiveBeginPlay`
  (`KismetSystemLibrary.K2_SetTimerDelegate` (delegate `MainTimerEvent`) 2.0 true))

(event `MainTimerEvent`
  (bind _result (`/Engine/EditorBlueprintResources/StandardMacros.IncrementInt` (`self.TimePlayed`))
    (:`  `
      (bind _returnvalue (cast `/Game/Blueprints/Light/ELightColor` (`KismetMathLibrary.Conv_IntToByte` (mod (+ _result (`self.ColorIndex`)) (`BlueprintMapLibrary.Map_Length` (`self.ColorMap`))))))
      (`self.SetColor` (`BlueprintMapLibrary.Map_Find` (`self.ColorMap`) _returnvalue) (`BlueprintMapLibrary.Map_Find` (`self.ColorNameMap`) _returnvalue)))))

(fn `SetColor`
  (params (NewLightColor :type "LinearColor Structure") (NewLightColorName :type "Text (by ref)"))
  (`LightComponent.SetLightColor` (`self.PointLight`) NewLightColor true)
  (`TextRenderComponent.K2_SetText` (`self.TextRender`) NewLightColorName))

(fn `UserConstructionScript`)