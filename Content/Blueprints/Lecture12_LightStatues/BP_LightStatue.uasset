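; BP_LightStatue is a statue actor that can be lit or unlit, pairing a mesh with a point light.
; Switchon and SwitchOff events both call a shared Switcher function with a state and a material.
; Switcher stores IsOn, sets the light's visibility and swaps the statue mesh between emissive and plain materials.
; IsSwitchedOn exposes the current state to callers.
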(event `/Game/Blueprints/Lecture12_LightStatues/BPI_Switchable.SwitchOn`
  (`self.Switcher` true (`self.EmissiveStatueMaterial`)))

(event `/Game/Blueprints/Lecture12_LightStatues/BPI_Switchable.SwitchOff`
  (`self.Switcher` false (`self.StatueMaterial`)))

(fn `IsSwitchedOn`
  (returns (IsOn :type Boolean))
  (return (`self.IsOn`)))

(fn `UserConstructionScript`)