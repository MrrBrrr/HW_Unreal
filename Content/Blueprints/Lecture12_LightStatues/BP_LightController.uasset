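; Master light switch actor that opens a menu for controlling light statues while something overlaps it.
; BP_LightManager triggers creation of WBP_LightMenu, whose all-light switch is bound back to this actor's toggle.
; Toggling sets IsOn, signals enable or disable, and refreshes the menu's buttons, which are also seeded from each statue's state.
; Overlap shows the menu with mouse cursor; leaving removes all widgets and restores game-only input.
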(event `self.SwitchOn`
  ;[1 1 1] On action button press
  (`self.CallOnEnable`)
  (`/Game/UI/WBP_LightMenu.UpdateButtons` (`self.LightMenuWidget`) :!label _label)
  (`/Game/UI/WBP_LightMenu.CheckIfAllChecked` (`self.LightMenuWidget`)))

(event `self.SwitchOff`
  ;[1 1 1] On action button press
  (`self.CallOnDisable`)
  (goto _label))

(event `CreateLightMenu`
  ;[1 1 1] Called by BP_LightManager
  (bind _returnvalue (`|CreateWidget` "/Game/UI/WBP_LightMenu.WBP_LightMenu_C"))
  (bind _output_get (set `self.LightMenuWidget` _returnvalue))
  (add `/Game/UI/WBP_LightMenu.AllLightSwitch` _output_get (delegate `SwitchTheLight`))
  (`self.UpdateButtonStatus`))

(event `SwitchTheLight`
  ;[1 1 1] Called by BP_LightManager
  (bind _ison (`self.IsSwitchedOn`))
  (if _ison
    (`self.CallOnDisable`)
    (else
      (`self.CallOnEnable`)))
  (`self.UpdateButtonStatus`))

(event `self.ReceiveActorBeginOverlap`
  (params (OtherActor :type "Actor Object Reference"))
  ;[1 1 1] Spawn Menu and update buttons
  (`UserWidget.AddToViewport` (`self.LightMenuWidget`) 0)
  (`WidgetBlueprintLibrary.SetInputMode_GameAndUIEx` (`GameplayStatics.GetPlayerController` 0) null "DoNotLock" false)
  (set `PlayerController.bShowMouseCursor` true (`GameplayStatics.GetPlayerController` 0))
  (`/Game/UI/WBP_LightMenu.UpdateButtons` (`self.LightMenuWidget`)))

(event `self.ReceiveActorEndOverlap`
  (params (OtherActor :type "Actor Object Reference"))
  ;[1 1 1] Spawn Menu and update buttons
  (`WidgetLayoutLibrary.RemoveAllWidgets`)
  (`WidgetBlueprintLibrary.SetInputMode_GameOnly` (`GameplayStatics.GetPlayerController` 0))
  (set `PlayerController.bShowMouseCursor` false (`GameplayStatics.GetPlayerController` 0))
  (`/Game/UI/WBP_LightMenu.UpdateButtons` (`self.LightMenuWidget`)))

(fn `CallOnDisable`
  (set `self.IsOn` false)
  (`self.OnDisable`))

(fn `CallOnEnable`
  (set `self.IsOn` true)
  (`self.OnEnable`))

(fn `IsSwitchedOn`
  (returns (IsOn :type Boolean))
  (return (`self.IsOn`)))

(fn `Set Statues To Widget`
  (params (LightStatues :type "Array of /Game/Blueprints/Lecture12_LightStatues/BP_LightStatue Object Reference"))
  (`/Game/UI/WBP_LightMenu.Set Statues` (`self.LightMenuWidget`) LightStatues)
  (for (_array_element _array_index) LightStatues
    (bind _ison (`/Game/Blueprints/Lecture12_LightStatues/BP_LightStatue.IsSwitchedOn` _array_element))
    (`/Game/UI/WBP_LightMenu.UpdateButtonStatusByIndex` (`self.LightMenuWidget`) _ison _array_index)
    (`/Game/UI/WBP_LightMenu.CheckIfAllChecked` (`self.LightMenuWidget`))))

(fn `UpdateButtonStatus`
  (bind _ison (`self.IsSwitchedOn`))
  (if _ison
    (`/Game/UI/WBP_LightMenu.ChangeAllLightButtonStatus` (`self.LightMenuWidget`) true)
    (else
      (`/Game/UI/WBP_LightMenu.ChangeAllLightButtonStatus` (`self.LightMenuWidget`) false))))

(fn `UserConstructionScript`)