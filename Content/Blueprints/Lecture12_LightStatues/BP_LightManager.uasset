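; Manager that sets up the light statues and links them to a LightController for enabling and disabling.
; On BeginPlay it has the controller create the light menu, then spawns two rows of three BP_LightStatue actors, flipping Y for the second row.
; Each spawned statue and the pre-placed table statue is subscribed to the controller's OnEnable and OnDisable events.
; The collected statue array is then passed to the controller's widget.
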(event `self.ReceiveBeginPlay`
  (`/Game/Blueprints/Lecture12_LightStatues/BP_LightController.CreateLightMenu` (`self.LightController`))
  (`self.SubsribeLightStatue` (`self.LightStatueOnTheTable`))
  (for _index (range 2)
    (if (not (== _index 0))
      (bind _output_get (set `self.PositionY` (* (`self.PositionY`) -1))))
    (for _index_2 (range 3)
      (bind _returnvalue (`|SpawnActorFromClass` "/Game/Blueprints/Lecture12_LightStatues/BP_LightStatue.BP_LightStatue_C" (`KismetMathLibrary.MakeTransform` (`KismetMathLibrary.MakeVector` (`KismetMathLibrary.Conv_IntToDouble` (* _index_2 400)) (`KismetMathLibrary.Conv_IntToDouble` _output_get))) "Undefined" "OverrideRootScale" null null))
      (`self.SubsribeLightStatue` _returnvalue)
      (`KismetArrayLibrary.Array_Add` (`self.SpannedLightStatues`) _returnvalue)))
  ;[1 1 1] Init Array for UI elements
  (`KismetArrayLibrary.Array_Add` (`self.SpannedLightStatues`) (`self.LightStatueOnTheTable`))
  (`/Game/Blueprints/Lecture12_LightStatues/BP_LightController.Set Statues To Widget` (`self.LightController`) (`self.SpannedLightStatues`)))

(fn `SubsribeLightStatue`
  (params (LightStatue :type "/Game/Blueprints/Lecture12_LightStatues/BP_LightStatue Object Reference"))
  ;[1 1 1] Subscribe  to controller
  (add `/Game/Blueprints/Lecture12_LightStatues/BP_LightController.OnEnable` (`self.LightController`) (`|CreateDelegate` LightStatue :!event `SwitchOn`))
  (add `/Game/Blueprints/Lecture12_LightStatues/BP_LightController.OnDisable` (`self.LightController`) (`|CreateDelegate` LightStatue :!event `SwitchOff`)))

(fn `UserConstructionScript`)