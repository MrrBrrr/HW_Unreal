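; BP_Teleport is a trigger actor that teleports BP_FemaleCharacter to the location of its Destination reference.
; Overlap plays a slap sound, sets a flag and starts a one-second retriggerable delay; end overlap clears the flag.
; The teleport runs only if the flag is still set after the delay, resetting rotation to zero.
; An invalid Destination sends the character to a fixed point above the world origin.
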(event `self.ReceiveActorBeginOverlap`
  (params (OtherActor :type "Actor Object Reference"))
  (bind _destination (`self.Destination`))
  (bind _asbp_female_character (cast `/Game/ThirdPersonBP/Blueprints/BP_FemaleCharacter` OtherActor))
  (`GameplayStatics.PlaySound2D` "/Game/Audio/Slap1.Slap1" 1.0 1.0 0.0 null null)
  (set `self.IsActorOverlapped` true)
  (`KismetSystemLibrary.RetriggerableDelay` 1.0)
  (if (`self.IsActorOverlapped`)
    (if (`KismetSystemLibrary.IsValid` _destination)
      (`self.K2_TeleportTo` :`self` _asbp_female_character :`DestLocation` (`self.K2_GetActorLocation` _destination))
      (else
        (`self.K2_TeleportTo` :`self` _asbp_female_character :`DestLocation` (0.0 0.0 100.0))))))

(event `self.ReceiveActorEndOverlap`
  (params (OtherActor :type "Actor Object Reference"))
  (cast `/Game/ThirdPersonBP/Blueprints/BP_FemaleCharacter` OtherActor)
  (set `self.IsActorOverlapped` false))

(fn `UserConstructionScript`)