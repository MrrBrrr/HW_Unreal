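; Scout actor that endlessly moves forward toward randomly placed BP_Projectile markers, replacing each target when it bumps into it.
; Targets spawn within X/Y bounds or, with IsAIMovement, at random reachable navigation points, flattened to the mesh's height.
; A per-tick line trace not hitting a projectile, or a frontal hit with another actor, spawns a recolored bypass marker.
; Reaching that bypass turns the mesh back to the main target.
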(event `self.ReceiveBeginPlay`
  (`self.GenerateAimActor`))

(event `self.ReceiveTick`
  (params (DeltaSeconds :type "Float (single-precision)"))
  (`self.MoveForward` DeltaSeconds)
  (`self.Draw Trace` (`self.CurrentAimTarget Location`)))

(event `self.ReceiveHit`
  (params (MyComp :type "PrimitiveComponent Object Reference") (Other :type "Actor Object Reference") (OtherComp :type "PrimitiveComponent Object Reference") (bSelfMoved :type Boolean) (HitLocation :type "Vector Structure") (HitNormal :type "Vector Structure") (NormalImpulse :type "Vector Structure") (Hit :type "HitResult Structure (by ref)"))
  ;[1 1 1] Prevent push from behind
  (if (> (`self.AngleBetweenVectors` HitNormal (`self.GetActorForwardVector`)) 90.0)
    (`self.ChangeDestination` Other)))

(fn `AngleBetweenVectors`
  (params (VectorA :type "Vector Structure") (VectorB :type "Vector Structure"))
  (returns (AngleInDegrees :type "Float (double-precision)"))
  (return (`KismetMathLibrary.DegAcos` (`KismetMathLibrary.Dot_VectorVector` (`KismetMathLibrary.Normal` VectorA 0.1) (`KismetMathLibrary.Normal` VectorB 0.1)))))

(fn `ChangeDestination`
  (params (OtherActor :type "Object Object Reference"))
  (if (== OtherActor (`self.AimActor`))
    (`self.GenerateAimActor`)
    (elif (`self.CompareToBypassAimActor` OtherActor)
      (`self.Rotate to Aim`)
      (else
        (bind _returnvalue (`self.ChooseAnotherWay`))
        (`self.RotateToTheTarget` _returnvalue)
        (set `self.CurrentAimTarget Location` (`self.IgnoreZ` (`self.K2_GetActorLocation` (`self.BypassAimActor`))))))))

(fn `ChooseAnotherWay`
  (returns (ReturnValue :type "Vector Structure"))
  (`/Engine/EditorBlueprintResources/StandardMacros.IsValid` (`self.BypassAimActor`)
    (:`Is Valid`
      (`self.K2_DestroyActor` (`self.BypassAimActor`)))
    (:`Is Not Valid`
      _))
  (bind _returnvalue (`|SpawnActorFromClass` "/Game/Blueprints/Lecture15_Scout/BP_Projectile.BP_Projectile_C" (`KismetMathLibrary.MakeTransform` (`self.IgnoreZ` (`NavigationSystemV1.K2_GetRandomReachablePointInRadius` (`self.K2_GetActorLocation`) 1000.0 null null)) (struct) (0.3 0.3 0.3)) "Undefined" "OverrideRootScale" null null))
  (bind _output_get (set `self.BypassAimActor` _returnvalue))
  (bind _staticmesh (`/Game/Blueprints/Lecture15_Scout/BP_Projectile.StaticMesh` _output_get))
  (`PrimitiveComponent.SetMaterial` _staticmesh 0 "/Engine/VREditor/UI/DiscMaterial.DiscMaterial")
  (return (`self.IgnoreZ` (`SceneComponent.K2_GetComponentLocation` _staticmesh))))

(fn `CompareToBypassAimActor`
  (params (Other :type "Object Object Reference"))
  (returns (ReturnValue :type Boolean))
  (return (and (`KismetSystemLibrary.IsValid` (`self.BypassAimActor`)) (== Other (`self.BypassAimActor`)))))

(fn `Destroy if Valid`
  (params (Object :type "Object Object Reference"))
  (if (`KismetSystemLibrary.IsValid` Object)
    (`self.K2_DestroyActor` (`self.AimActor`))
    (return)
    (else
      (return))))

(fn `Draw Trace`
  (params (`Target Location` :type "Vector Structure"))
  (bind _outhit (`KismetSystemLibrary.LineTraceSingleForObjects` :`Start` (`SceneComponent.K2_GetComponentLocation` (`self.StaticMesh`)) :`End` `Target Location` :`ObjectTypes` (`self.Object Types`) :`DrawDebugType` "ForOneFrame"))
  (bind _asbp_projectile (cast `/Game/Blueprints/Lecture15_Scout/BP_Projectile` (`.HitActor` (`GameplayStatics.BreakHitResult` _outhit)))
    (:`CastFailed`
      (`self.ChangeDestination` _asbp_projectile))))

(fn `GenerateAimActor`
  (bind _aimspawnlocation (`self.Set Next Random Target`))
  (bind _output_get (set `self.CurrentAimTarget Location` _aimspawnlocation))
  (`self.RotateToTheTarget` _output_get))

(fn `IgnoreZ`
  (params (InputVector :type "Vector Structure"))
  (returns (OutputVector :type "Vector Structure"))
  (bind (_returnvalue_x _returnvalue_y _returnvalue_z) (`KismetMathLibrary.BreakVector` (`SceneComponent.K2_GetComponentLocation` (`self.StaticMesh`))))
  (return (`KismetMathLibrary.MakeVector` InputVector_X InputVector_Y _returnvalue_z)))

(fn `MoveForward`
  (params (Delta :type "Float (double-precision)"))
  (`self.K2_AddActorWorldOffset` (* (`self.GetActorForwardVector`) (* Delta (`self.Speed`))) true))

(fn `Rotate to Aim`
  (bind _outputvector (`self.IgnoreZ` (`self.K2_GetActorLocation` (`self.AimActor`))))
  (`self.K2_DestroyActor` (`self.BypassAimActor`))
  (`self.RotateToTheTarget` _outputvector)
  (set `self.CurrentAimTarget Location` _outputvector))

(fn `RotateToTheTarget`
  (params (Target :type "Vector Structure (by ref)"))
  (`SceneComponent.K2_SetWorldRotation` (`self.StaticMesh`) (`KismetMathLibrary.FindLookAtRotation` (`SceneComponent.K2_GetComponentLocation` (`self.StaticMesh`)) Target) false false))

(fn `Set Next Random Target`
  (returns (AimSpawnLocation :type "Vector Structure"))
  (locals (AimActorSpawnLocation :type "Vector Structure" :default (0.0 0.0 0.0)))
  (`self.Destroy if Valid` (`self.AimActor`))
  (if (not (`self.IsAIMovement`))
    (set `local.AimActorSpawnLocation` (`self.IgnoreZ` (`KismetMathLibrary.MakeVector` (`KismetMathLibrary.RandomFloatInRange` (`self.Min X`) (`self.Max X`)) (`KismetMathLibrary.RandomFloatInRange` (`self.Min Y`) (`self.Max Y`)))))
    (else
      (set `local.AimActorSpawnLocation` (`self.IgnoreZ` (`NavigationSystemV1.K2_GetRandomReachablePointInRadius` (`self.K2_GetActorLocation`) 1000.0 null null)))))
  (bind _returnvalue (`|SpawnActorFromClass` "/Game/Blueprints/Lecture15_Scout/BP_Projectile.BP_Projectile_C" (`KismetMathLibrary.MakeTransform` (`local.AimActorSpawnLocation`) (struct) (0.3 0.3 0.3)) "Undefined" "OverrideRootScale" null null))
  (set `self.AimActor` _returnvalue)
  (return (`local.AimActorSpawnLocation`)))

(fn `UserConstructionScript`)